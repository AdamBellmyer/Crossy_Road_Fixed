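; Moving vehicle obstacle for a Crossy Road style game that ends the game when it hits the player.
; Each tick it offsets itself along its root's right vector by Speed, without scaling by delta time, so movement is frame-rate dependent.
; Once farther than Distance from StartPos it teleports back there, looping the same actor.
; Overlapping a player_bp calls that player's GameOver.
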(event EventTick
  (params (DeltaSeconds :type Float%20%28single-precision%29))
  (Transformation|AddActorWorldOffset (* (Math|Vector|GetRightVector (Variables|Default|GetDefaultSceneRoot)) (Variables|Default|Getspeed)))
  (if (> (Math|Vector|Distance(Vector) (Transformation|GetActorLocation) (Variables|Default|GetstartPos)) (Variables|Default|Getdistance))
    (Transformation|SetActorLocation (Variables|Default|GetstartPos) false false)))

(event Collision|EventActorBeginOverlap
  (params (OtherActor :type Actor%20Object%20Reference))
  (bind _asplayer_bp (Utilities|Casting|CastToplayer_bp OtherActor))
  (Default|GameOver _asplayer_bp))

(fn ConstructionScript)