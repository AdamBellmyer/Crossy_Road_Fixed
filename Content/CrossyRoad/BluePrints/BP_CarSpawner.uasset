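; BP_CarSpawner is a Crossy Road actor that spawns BP_Vehicle cars, starting with one at the world origin on BeginPlay.
; SpawnVehicle creates the car at a given location and stores it as NewCar.
; SpawnCarAtSpawnPoint spawns another at the stored car's current location, not the spawner's, and is not called within this Blueprint.
; The node that would set the car's VehicleSpawner back-reference is unconnected, so it never runs.
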(event EventBeginPlay
  (CallFunction|SpawnVehicle "0.000000,0.000000,0.000000"))

(event Collision|EventActorBeginOverlap
  (params (OtherActor :type Actor%20Object%20Reference)))

(event EventTick
  (params (DeltaSeconds :type Float%20%28single-precision%29)))

(fn ConstructionScript)

(fn SpawnVehicle
  (params (Spawn%20Location :type Vector))
  (bind _returnvalue (Game|SpawnActorfromClass "/Game/CrossyRoad/BluePrints/BP_Vehicle.BP_Vehicle_C" (Math|Transform|MakeTransform Spawn%20Location "0, 0, 0" "1,1,1") "Undefined" 0 0))
  (bind _output_get (Variables|Default|SetNew%20Car _returnvalue)))

(fn SpawnCaratSpawnPoint
  (CallFunction|SpawnVehicle (Transformation|GetWorldLocation (Variables|/Script/Engine.Actor|GetRootComponent (Variables|Default|GetNew%20Car)))))